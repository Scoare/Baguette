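; Player controller logic for a French-language baguette-baking game where the player feeds a hungry chef to survive until time runs out.
; Mouse traces dispatch on actor tags to drag items between crates, bowls, fridge, oven and chef, or open measuring, mixing, shaping and timer widgets.
; IsStunned blocks interaction during widgets and dialogue, while TutorialState advances onboarding.
; Baguette ingredient ratings adjust Hunger, which a timer drains toward Lose or Win levels.
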(event `self.ReceiveBeginPlay`
  (set `self.bShowMouseCursor` true)
  (message `EnhancedInputSubsystemInterface.AddMappingContext` (subsystem `EnhancedInputLocalPlayerSubsystem`) "/Game/Input/PlayerInputMappingContext.PlayerInputMappingContext" 0 (struct))
  (`self.InitiateTooltipUI`)
  (`self.InitiateErrorLogUI`)
  (`self.InitiateDialogue` (`|MakeArray` "Hmmm... bonjour... il semble que notre dernier employé été... *sniff* licencié. Tu es ici pour lui remplacer maintenant." "Mais, ne vous inquiétez pas, le travail est très simple." "Pour commencer, sortez quelques ingrédients de ces boîtes et mesurez-les." "Vous pouvez faire glisser les ingrédients avec votre souris pour les déplacer. (Tenir le clic gauche)" "Vous pouvez les mesurer par maintener votre souris dessus et en appuyant sur le bouton droit.")))

(event `EnhancedInput|/Game/Input/LeftClick`
  (params (ActionValue :type Boolean) (ElapsedSeconds :type "Float (double-precision)") (TriggeredSeconds :type "Float (double-precision)") (InputAction :type "InputAction Object Reference" :default "/Game/Input/LeftClick.LeftClick"))
  (bind _objectheld (`self.ObjectHeld`))
  (bind _returnvalue (`KismetSystemLibrary.IsValid` _objectheld))
  (bind _returnvalue_2 (or (`self.ActorHasTag` _objectheld "Baguette") (`self.ActorHasTag` _objectheld "Dough")))
  (:`Started`
    (bind (_hitresult _didhit) (`self.RayTraceFromMouse` _))
    (if _didhit
      (bind (_bblockinghit _binitialoverlap _time _distance _location _impactpoint _normal _impactnormal _physmat _hitactor) (`GameplayStatics.BreakHitResult` _hitresult))
      (if (`self.ActorHasTag` _hitactor "Item")
        (`self.PickUpObject` _hitresult)
        (elif (`self.ActorHasTag` _hitactor "Bowl")
          (`self.PickUpDough` _hitresult)
          (elif (`self.ActorHasTag` _hitactor "Fridge")
            (bind _asbp_fridge (cast `/Game/Blueprints/BP_Fridge` _hitactor))
            (bind _currentobject (`/Game/Blueprints/BP_Fridge.CurrentObject` _asbp_fridge))
            (set `self.ObjectHeld` _currentobject)
            (bind _asbp_dough_item (cast `/Game/Blueprints/Items/BP_DoughItem` _currentobject)
              (:`then`
                (bind _returnvalue_3 (`self.GetComponentByClass` _asbp_dough_item "/Script/Engine.StaticMeshComponent"))
                (bind _returnvalue_x (`KismetMathLibrary.BreakVector` (`SceneComponent.K2_GetComponentScale` _returnvalue_3)))
                (bind _returnvalue_4 (`KismetMathLibrary.FClamp` (* (/ (`/Game/Blueprints/Items/BP_ItemBase.TimeInFridge` _asbp_dough_item) 6) _returnvalue_x) 0.5 2.0))
                (`SceneComponent.SetWorldScale3D` _returnvalue_3 (`KismetMathLibrary.MakeVector` _returnvalue_4 _returnvalue_4 _returnvalue_4)))
              (:`CastFailed`
                _))
            (set `/Game/Blueprints/BP_Fridge.CurrentObject` null _asbp_fridge)
            (elif (`self.ActorHasTag` _hitactor "Oven")
              (bind _asbp_oven (cast `/Game/Blueprints/BP_Oven` _hitactor))
              (set `self.ObjectHeld` (`/Game/Blueprints/BP_Oven.CurrentObject` _asbp_oven))
              (set `/Game/Blueprints/BP_Oven.CurrentObject` null _asbp_oven)
              (elif (`self.ActorHasTag` _hitactor "Crate")
                (if (not (`self.IsStunned`))
                  (`GameplayStatics.PlaySound2D` "/Game/Sounds/plop.plop" 1.0 1.0 0.0 null null)
                  (bind _asbp_crate (cast `/Game/Blueprints/BP_Crate` _hitactor))
                  (bind _returnvalue_5 (`|SpawnActorFromClass` (`/Game/Blueprints/BP_Crate.StoredItem` _asbp_crate) (`KismetMathLibrary.MakeTransform` _location) "Undefined" "MultiplyWithRoot" null null))
                  (`PrimitiveComponent.SetSimulatePhysics` (`/Game/Blueprints/Items/BP_ItemBase.Mesh` _returnvalue_5) false)
                  (set `self.ObjectHeld` _returnvalue_5)))))))))
  (:`Completed`
    (bind (_hitresult_2 _didhit_2) (`self.RayTraceFromMouse` _))
    (if _didhit_2
      (bind (_bblockinghit_2 _binitialoverlap_2 _time_2 _distance_2 _location_2 _impactpoint_2 _normal_2 _impactnormal_2 _physmat_2 _hitactor_2) (`GameplayStatics.BreakHitResult` _hitresult_2))
      (if (and (`self.ActorHasTag` _hitactor_2 "Fridge") _returnvalue)
        (if _returnvalue_2
          (`self.StoreInFridge` _hitresult_2)
          (else
            (if (`self.ActorHasTag` _hitactor_2 "Chef") :!label _label
              (`self.Chef` _hitresult_2)
              (else
                (`self.DropItem` :!label _label_2)))))
        (elif (and (`self.ActorHasTag` _hitactor_2 "Oven") _returnvalue)
          (if _returnvalue_2
            (`self.StoreInOven` _hitresult_2)
            (else
              (goto _label)))
          (else
            (goto _label))))
      (else
        (goto _label_2)))))

(event `self.ReceiveTick`
  (params (DeltaSeconds :type "Float (single-precision)"))
  (`self.MoveObject` DeltaSeconds)
  (`self.Tooltips`)
  (`self.BowlTooltips`))

(event `EnhancedInput|/Game/Input/RightClick`
  (params (ActionValue :type Boolean) (ElapsedSeconds :type "Float (double-precision)") (TriggeredSeconds :type "Float (double-precision)") (InputAction :type "InputAction Object Reference" :default "/Game/Input/RightClick.RightClick"))
  (:`Started`
    (bind _hitresult (`self.RayTraceFromMouse` _))
    (bind (_bblockinghit _binitialoverlap _time _distance _location _impactpoint _normal _impactnormal _physmat _hitactor) (`GameplayStatics.BreakHitResult` _hitresult))
    (if (`self.ActorHasTag` _hitactor "Item")
      (bind _returnvalue (`self.ActorHasTag` _hitactor "Dough"))
      (if _returnvalue
        (`self.InitiateShapingGame` _hitresult)
        (elif (not (or _returnvalue (`self.ActorHasTag` _hitactor "Baguette")))
          (`self.InitiateSlider` _hitactor)))
      (elif (`self.ActorHasTag` _hitactor "Bowl")
        (`self.InitiateBowlGame` _hitactor)
        (elif (`self.ActorHasTag` _hitactor "Clock")
          (`self.InitiateTimer` _hitresult))))))

(event `InitiateHungerTick`
  (`KismetSystemLibrary.K2_SetTimerDelegate` (delegate `HungerTick`) 1.0 true))

(event `HungerTick`
  (if (not (`self.Paused`))
    (bind _output_get (set `self.Hunger` (- (`self.Hunger`) 0.0075)))
    (bind _result (`/Engine/EditorBlueprintResources/StandardMacros.DecrementInt` (`self.TimeLeft`))
      (:`  `
        (if (<= _result 0)
          (`GameplayStatics.OpenLevelBySoftObjectPtr` "/Game/Levels/Win.Win")
          (elif (<= _output_get 0.0)
            (`GameplayStatics.OpenLevelBySoftObjectPtr` "/Game/Levels/Lose.Lose")))))))

(event `EnhancedInput|/Game/Input/Escape`
  (params (ActionValue :type Boolean) (ElapsedSeconds :type "Float (double-precision)") (TriggeredSeconds :type "Float (double-precision)") (InputAction :type "InputAction Object Reference" :default "/Game/Input/Escape.Escape"))
  (:`Started`
    (if (and (not (`self.Paused`)) (not (`self.IsStunned`)))
      (set `self.Paused` true)
      (set `self.IsStunned` true)
      (bind _returnvalue (`|CreateWidget` "/Game/Widgets/BP_Pause.BP_Pause_C"))
      (`UserWidget.AddToViewport` _returnvalue 0))))

(event `DespawnParticles`
  (params (Particles :type "ParticleSystemComponent Object Reference"))
  (`KismetSystemLibrary.Delay` 2.0)
  (`ActorComponent.Deactivate` Particles))

(fn `BowlTooltips`
  (locals (TempNameFrench :type String))
  (bind (_locationx _locationy) (`self.GetMousePosition`))
  (bind _bowltooltip (`self.BowlTooltip`))
  (bind _returnvalue (`PanelWidget.GetAllChildren` (`/Game/Widgets/BP_BowlTooltip.VerticalBox_434` _bowltooltip)))
  (bind (_hitresult _didhit) (`self.RayTraceFromMouse` _))
  (if (and _didhit (not (`self.IsStunned`)))
    (bind (_bblockinghit _binitialoverlap _time _distance _location _impactpoint _normal _impactnormal _physmat _hitactor) (`GameplayStatics.BreakHitResult` _hitresult))
    (if (`self.ActorHasTag` _hitactor "Bowl")
      (bind _asbp_bowl (cast `/Game/Blueprints/BP_Bowl` _hitactor))
      (`Widget.SetVisibility` _bowltooltip "Visible")
      (for (_array_element _array_index) _returnvalue
        (if (!= _array_index 0)
          (bind _astext (cast `TextBlock` _array_element))
          (bind _amounts (`/Game/Blueprints/BP_Bowl.Amounts` _asbp_bowl))
          (bind _keys (`BlueprintMapLibrary.Map_Keys` _amounts))
          (switch `string` (`|GetArrayItem` _keys (+ _array_index -1))
            (:`Flour`
              (set `local.TempNameFrench` "Farine"))
            (:`Honey`
              (set `local.TempNameFrench` "Miel"))
            (:`Salt`
              (set `local.TempNameFrench` "Sel"))
            (:`Water`
              (set `local.TempNameFrench` "Eau"))
            (:`Yeast`
              (set `local.TempNameFrench` "Levure")))
          (set `TextBlock.Text` (`KismetTextLibrary.Conv_StringToText` (`KismetStringLibrary.Concat_StrStr` (`local.TempNameFrench`) ": " (`KismetTextLibrary.Conv_TextToString` (`KismetTextLibrary.Conv_IntToText` (`BlueprintMapLibrary.Map_Find` _amounts (`KismetSystemLibrary.GetObjectName` _array_element)))) " grammes")) _astext)))
      (for _array_element_2 _returnvalue
        (bind _astext_2 (cast `TextBlock` _array_element_2))
        (if (`KismetTextLibrary.EqualEqual_TextText` (`TextBlock.Text` _astext_2) (`KismetTextLibrary.Conv_IntToText` 0))
          (`Widget.SetVisibility` _array_element_2 "Hidden")
          (else
            (`Widget.SetVisibility` _array_element_2 "Visible"))))
      (`UserWidget.SetPositionInViewport` _bowltooltip (`KismetMathLibrary.MakeVector2D` _locationx _locationy) true)
      (else
        (`Widget.SetVisibility` _bowltooltip "Hidden" :!label _label)))
    (else
      (goto _label))))

(fn `Chef`
  (params (Hit :type "HitResult Structure"))
  (bind _objectheld (`self.ObjectHeld`))
  (if (`KismetSystemLibrary.IsValid` _objectheld)
    (if (`self.ActorHasTag` _objectheld "Baguette")
      (bind _asbp_baguette_item (cast `/Game/Blueprints/Items/BP_BaguetteItem` _objectheld))
      (`GameplayStatics.PlaySound2D` "/Game/Sounds/eat.eat" 1.0 1.0 0.0 null null)
      (`self.EvaluateBaguette` _asbp_baguette_item)
      (bind _asbp_chef (cast `/Game/Blueprints/BP_Chef` Hit_HitActor))
      (bind _particlesystem (`/Game/Blueprints/BP_Chef.ParticleSystem` _asbp_chef))
      (`ActorComponent.Activate` _particlesystem false)
      (`self.DespawnParticles` _particlesystem)
      (`self.K2_DestroyActor` _objectheld)
      (switch `/Game/Blueprints/Player/TutorialEnum` (`self.TutorialState`)
        (:`NewEnumerator9`
          (`self.InitiateDialogue` (`|MakeArray` "Bien.. vous êtes prêt à faire des baguettes.." "N'oubliez pas que vous pouvez regarder l'affiche pour de l'aide. Maintenant.." "J'AI FAIM.. JE VEUX DES B A G U E T T E S !!!") true 2 0.1)
          (set `self.TutorialState` "NewEnumerator14")))
      (else
        (`self.DropItem`)))))

(fn `DropItem`
  (bind _objectheld (`self.ObjectHeld`))
  (if (`KismetSystemLibrary.IsValid` _objectheld)
    (`PrimitiveComponent.SetSimulatePhysics` (`self.GetComponentByClass` _objectheld "/Script/Engine.StaticMeshComponent") true)
    (`self.SetActorEnableCollision` _objectheld true)
    (set `self.ObjectHeld` null)))

(fn `EvaluateBaguette`
  (params (Baguette :type "/Game/Blueprints/Items/BP_BaguetteItem Object Reference"))
  (bind _amounts (`/Game/Blueprints/Items/BP_BaguetteItem.Amounts` Baguette))
  (bind _evaluationstandards (`self.EvaluationStandards`))
  (bind _keys (`BlueprintMapLibrary.Map_Keys` _amounts))
  (bind _values (`BlueprintMapLibrary.Map_Values` _amounts))
  (`BlueprintMapLibrary.Map_Keys` _evaluationstandards)
  (bind _values_2 (`BlueprintMapLibrary.Map_Values` _evaluationstandards))
  (for (_ _array_index) _keys
    (`self.EvaluateThing` (`KismetMathLibrary.Conv_IntToDouble` (`|GetArrayItem` _values _array_index)) (`KismetMathLibrary.Conv_IntToDouble` (`|GetArrayItem` _values_2 _array_index)))))

(fn `EvaluateThing`
  (params (ActualValue :type "Float (double-precision)") (ExpectedValue :type "Float (double-precision)"))
  (bind _returnvalue (* ExpectedValue 1.25))
  (bind _returnvalue_2 (* ExpectedValue 0.75))
  (bind _hunger (`self.Hunger`))
  (if (> ActualValue _returnvalue)
    (set `self.Hunger` (`KismetMathLibrary.FClamp` (- _hunger (/ (- ActualValue _returnvalue) 10000.0))))
    (elif (< ActualValue _returnvalue_2)
      (set `self.Hunger` (`KismetMathLibrary.FClamp` (- _hunger (/ (- _returnvalue_2 ActualValue) 10000.0))))
      (else
        (set `self.Hunger` (`KismetMathLibrary.FClamp` (+ _hunger 0.015)))))))

(fn `InitiateBowlGame`
  (params (BowlActor :type "Actor Object Reference"))
  (locals (HasIngredients :type Boolean :default true))
  (if (not (`self.IsStunned`))
    (bind _asbp_bowl (cast `/Game/Blueprints/BP_Bowl` BowlActor))
    (bind _values (`BlueprintMapLibrary.Map_Values` (`/Game/Blueprints/BP_Bowl.Amounts` _asbp_bowl)))
    (for _array_element _values
      (if (== _array_element 0)
        (set `local.HasIngredients` false)
        (`self.LogError` "Il manque des ingrédients")
        (break)))
    (if (`local.HasIngredients`)
      (set `self.IsStunned` true)
      (bind _returnvalue (`|CreateWidget` "/Game/Widgets/BP_MixingGame.BP_MixingGame_C"))
      (`UserWidget.AddToViewport` _returnvalue 0)
      (set `/Game/Widgets/BP_MixingGame.Bowl` _asbp_bowl _returnvalue)
      (`/Game/Widgets/BP_MixingGame.ButtonClicked` _returnvalue))))

(fn `InitiateDialogue`
  (params (Dialogue :type "Array of String") (ShouldCameraShake :type Boolean) (CameraStartShakingOn :type Integer :default 0) (Speed :type "Float (double-precision)" :default 0.0))
  (set `self.IsStunned` true)
  (bind _returnvalue (`|CreateWidget` "/Game/Widgets/BP_Dialogue.BP_Dialogue_C"))
  (`UserWidget.AddToViewport` _returnvalue 0)
  (set `/Game/Widgets/BP_Dialogue.Dialogues` Dialogue _returnvalue)
  (set `/Game/Widgets/BP_Dialogue.PlayCameraShake` ShouldCameraShake _returnvalue)
  (set `/Game/Widgets/BP_Dialogue.StartShakingOn` CameraStartShakingOn _returnvalue)
  (set `/Game/Widgets/BP_Dialogue.TypeSpeed` Speed _returnvalue)
  (`/Game/Widgets/BP_Dialogue.Ready` _returnvalue))

(fn `InitiateErrorLogUI`
  (bind _returnvalue (`|CreateWidget` "/Game/Widgets/BP_ErrorLog.BP_ErrorLog_C"))
  (bind _output_get (set `self.ErrorLog` _returnvalue))
  (`UserWidget.AddToViewport` _output_get 0))

(fn `InitiateShapingGame`
  (params (Hit :type "HitResult Structure"))
  (bind _asbp_dough_item (cast `/Game/Blueprints/Items/BP_DoughItem` (`.HitActor` (`GameplayStatics.BreakHitResult` Hit))))
  (if (and (not (`self.IsStunned`)) (< (`/Game/Blueprints/Items/BP_ItemBase.TimeInOven` _asbp_dough_item) 0.5))
    (switch `/Game/Blueprints/Player/TutorialEnum` (`self.TutorialState`)
      (:`NewEnumerator12`
        _)
      (:`NewEnumerator11`
        _)
      (:`NewEnumerator9`
        _)
      (:`NewEnumerator14`
        _))
    (set `self.IsStunned` true)
    (bind _returnvalue (`|CreateWidget` "/Game/Widgets/BP_RollingGame.BP_RollingGame_C"))
    (`UserWidget.AddToViewport` _returnvalue 0)
    (set `/Game/Widgets/BP_RollingGame.Dough` _asbp_dough_item _returnvalue)))

(fn `InitiateSlider`
  (params (ItemActor :type "Actor Object Reference"))
  (if (not (`self.IsStunned`))
    (set `self.IsStunned` true)
    (bind _returnvalue (`|CreateWidget` "/Game/Widgets/BP_AmountSlider.BP_AmountSlider_C"))
    (`UserWidget.AddToViewport` _returnvalue 0)
    (bind _asbp_item_base (cast `/Game/Blueprints/Items/BP_ItemBase` ItemActor))
    (`Slider.SetMaxValue` (`/Game/Widgets/BP_AmountSlider.Slider_87` _returnvalue) (`KismetMathLibrary.Conv_IntToDouble` (`/Game/Blueprints/Items/BP_ItemBase.Amount` _asbp_item_base)))
    (set `/Game/Widgets/BP_AmountSlider.Item` _asbp_item_base _returnvalue)))

(fn `InitiateTimer`
  (params (Hit :type "HitResult Structure"))
  (bind _asbp_clock (cast `/Game/Blueprints/BP_Clock` (`.HitActor` (`GameplayStatics.BreakHitResult` Hit))))
  (if (not (`self.IsStunned`))
    (set `self.IsStunned` true)
    (bind _returnvalue (`|CreateWidget` "/Game/Widgets/BP_AmountSliderTime.BP_AmountSliderTime_C"))
    (`UserWidget.AddToViewport` _returnvalue 0)
    (set `/Game/Widgets/BP_AmountSliderTime.ClockActor` _asbp_clock _returnvalue)))

(fn `InitiateTooltipUI`
  (bind _returnvalue (`|CreateWidget` "/Game/Widgets/BP_AmountTooltip.BP_AmountTooltip_C"))
  (bind _output_get (set `self.Tooltip` _returnvalue))
  (`UserWidget.AddToViewport` _output_get 0)
  (bind _returnvalue_2 (`|CreateWidget` "/Game/Widgets/BP_BowlTooltip.BP_BowlTooltip_C"))
  (bind _output_get_2 (set `self.BowlTooltip` _returnvalue_2))
  (`UserWidget.AddToViewport` _output_get_2 0))

(fn `LogError`
  (params (Message :type String :default "Hello World!") (Type :type "/Game/Blueprints/Player/ErrorLogEnum Enum" :default "NewEnumerator2") (Time :type "Float (double-precision)" :default 5.0))
  (bind _returnvalue (`|CreateWidget` "/Game/Widgets/BP_ErrorMessage.BP_ErrorMessage_C"))
  (`PanelWidget.AddChild` (`/Game/Widgets/BP_ErrorLog.VerticalBox_434` (`self.ErrorLog`)) _returnvalue)
  (set `/Game/Widgets/BP_ErrorMessage.Time` Time _returnvalue)
  (set `TextBlock.Text` (`KismetTextLibrary.Conv_StringToText` Message) (`/Game/Widgets/BP_ErrorMessage.TextBlock_169` _returnvalue))
  (switch `/Game/Blueprints/Player/ErrorLogEnum` Type
    (:`NewEnumerator0`
      (bind _textblock_169 (`/Game/Widgets/BP_ErrorMessage.TextBlock_169` _returnvalue))
      (set `TextBlock.ColorAndOpacity` (make `SlateColor` (struct :`R` 1.0 :`A` 1.0)) _textblock_169))
    (:`NewEnumerator1`
      (set `TextBlock.ColorAndOpacity` (make `SlateColor` (struct :`R` 1.0 :`G` 1.0 :`A` 1.0)) _textblock_169))
    (:`NewEnumerator2`
      (set `TextBlock.ColorAndOpacity` (make `SlateColor` (struct :`R` 1.0 :`G` 1.0 :`B` 1.0 :`A` 1.0)) _textblock_169))))

(fn `MoveObject`
  (params (DeltaTime :type "Float (double-precision)"))
  (bind (_minposition_x _minposition_y _minposition_z) (`KismetMathLibrary.BreakVector` (`self.MinPosition`)))
  (bind _objectheld (`self.ObjectHeld`))
  (bind (_maxposition_x _maxposition_y _maxposition_z) (`KismetMathLibrary.BreakVector` (`self.MaxPosition`)))
  (if (and (`KismetSystemLibrary.IsValid` _objectheld) (not (`self.IsStunned`)))
    (bind _hitresult (`self.RayTraceFromMouse` (`|MakeArray` _objectheld)))
    (bind (_returnvalue_x _returnvalue_y _returnvalue_z) (`KismetMathLibrary.BreakVector` (`KismetMathLibrary.VInterpTo` (`self.K2_GetActorLocation` _objectheld) (+ (`.Location` (`GameplayStatics.BreakHitResult` _hitresult)) (0.0 0.0 250.0)) DeltaTime 5.0)))
    (`self.K2_SetActorLocation` _objectheld (`KismetMathLibrary.MakeVector` (`KismetMathLibrary.FClamp` _returnvalue_x _minposition_x _maxposition_x) (`KismetMathLibrary.FClamp` _returnvalue_y _minposition_y _maxposition_y) (`KismetMathLibrary.FClamp` _returnvalue_z _minposition_z _maxposition_z)) false false)
    (else
      (`self.DropItem`))))

(fn `PickUpDough`
  (params (Hit :type "HitResult Structure"))
  (bind (_bblockinghit _binitialoverlap _time _distance _location _impactpoint _normal _impactnormal _physmat _hitactor) (`GameplayStatics.BreakHitResult` Hit))
  (bind _asbp_bowl (cast `/Game/Blueprints/BP_Bowl` _hitactor))
  (if (`/Game/Blueprints/BP_Bowl.HasDough` _asbp_bowl)
    (set `/Game/Blueprints/BP_Bowl.HasDough` false _asbp_bowl)
    (bind _doughamounts (`/Game/Blueprints/BP_Bowl.DoughAmounts` _asbp_bowl))
    (bind _keys (`BlueprintMapLibrary.Map_Keys` _doughamounts))
    (bind _values (`BlueprintMapLibrary.Map_Values` _doughamounts))
    (bind _returnvalue (`|SpawnActorFromClass` "/Game/Blueprints/Items/BP_DoughItem.BP_DoughItem_C" (`KismetMathLibrary.MakeTransform` _location) "Undefined" "MultiplyWithRoot" null null))
    (for (_array_element _array_index) _keys
      (bind _output (`|GetArrayItem` _values _array_index))
      (`BlueprintMapLibrary.Map_Add` (`/Game/Blueprints/Items/BP_DoughItem.DoughAmounts` _returnvalue) _array_element _output)
      (set `/Game/Blueprints/Items/BP_ItemBase.Amount` (+ (`/Game/Blueprints/Items/BP_ItemBase.Amount` _returnvalue) _output) _returnvalue)
      (`BlueprintMapLibrary.Map_Remove` _doughamounts _array_element)
      (`BlueprintMapLibrary.Map_Add` _doughamounts _array_element))
    (`SceneComponent.SetVisibility` (`/Game/Blueprints/BP_Bowl.stuff_in_bowl` _asbp_bowl) false false)
    (set `self.ObjectHeld` _returnvalue)
    (`PrimitiveComponent.SetSimulatePhysics` (`/Game/Blueprints/Items/BP_ItemBase.Mesh` _returnvalue) false)
    (bind _returnvalue_2 (`KismetMathLibrary.FClamp` (/ (`KismetMathLibrary.Conv_IntToDouble` (`/Game/Blueprints/Items/BP_ItemBase.Amount` _returnvalue)) 898.0) 0.25))
    (`SceneComponent.SetWorldScale3D` (`self.GetComponentByClass` _returnvalue "/Script/Engine.StaticMeshComponent") (`KismetMathLibrary.MakeVector` _returnvalue_2 _returnvalue_2 _returnvalue_2))))

(fn `PickUpObject`
  (params (Hit :type "HitResult Structure"))
  (bind (_bblockinghit _binitialoverlap _time _distance _location _impactpoint _normal _impactnormal _physmat _hitactor _hitcomponent) (`GameplayStatics.BreakHitResult` Hit))
  (if (and (== (`SceneComponent.Mobility` _hitcomponent) 2) (not (`self.IsStunned`)))
    (set `self.ObjectHeld` _hitactor)
    (`PrimitiveComponent.SetSimulatePhysics` _hitcomponent false)
    (`self.SetActorEnableCollision` _hitactor false)))

(fn `RayTraceFromMouse`
  (params (ActorsToIgnore :type "Array of Actor Object Reference"))
  (returns (HitResult :type "HitResult Structure") (DidHit :type Boolean))
  (bind (_worldlocation _worlddirection) (`self.DeprojectMousePositionToWorld`))
  (bind (_outhit _returnvalue) (`KismetSystemLibrary.LineTraceSingle` _worldlocation (+ _worldlocation (* _worlddirection 10000.0)) "TraceTypeQuery1" false ActorsToIgnore))
  (return _outhit _returnvalue))

(fn `StoreInFridge`
  (params (Hit :type "HitResult Structure"))
  (bind _objectheld (`self.ObjectHeld`))
  (bind _asbp_fridge (cast `/Game/Blueprints/BP_Fridge` (`.HitActor` (`GameplayStatics.BreakHitResult` Hit))))
  (if (`KismetSystemLibrary.IsValid` _objectheld)
    (if (not (`KismetSystemLibrary.IsValid` (`/Game/Blueprints/BP_Fridge.CurrentObject` _asbp_fridge)))
      (set `/Game/Blueprints/BP_Fridge.CurrentObject` _objectheld _asbp_fridge)
      (for _array_element (`self.K2_GetComponentsByClass` _objectheld "/Script/Engine.StaticMeshComponent")
        (bind _asstatic_mesh_component (cast `StaticMeshComponent` _array_element))
        (`PrimitiveComponent.SetSimulatePhysics` _asstatic_mesh_component false)
        (`self.SetActorEnableCollision` _objectheld false))
      (set `self.ObjectHeld` null)
      (switch `/Game/Blueprints/Player/TutorialEnum` (`self.TutorialState`)
        (:`NewEnumerator8`
          (`self.InitiateDialogue` (`|MakeArray` "Maintenant, utilisez les horloges pour laisser fermenter la pâte pendant un certain temps. (clic droit)"))
          (set `self.TutorialState` "NewEnumerator10")
          (bind _returnvalue (`|SpawnActorFromClass` "/Game/Blueprints/BP_Clock.BP_Clock_C" (`KismetMathLibrary.MakeTransform` (1113.39398 215.278836 92.82303) (struct :`Yaw` 89.999999 :`Roll` -11.294349) (2.5 2.5 2.5)) "Undefined" "MultiplyWithRoot" null null))
          (set `/Game/Blueprints/BP_Clock.Mode` "NewEnumerator0" _returnvalue)
          (bind _returnvalue_2 (`|SpawnActorFromClass` "/Game/Blueprints/BP_Clock.BP_Clock_C" (`KismetMathLibrary.MakeTransform` (1113.39398 25.278836 36.781198) (struct :`Yaw` 89.999999 :`Roll` -11.294349)) "Undefined" "MultiplyWithRoot" null null))
          (set `/Game/Blueprints/BP_Clock.Mode` "NewEnumerator1" _returnvalue_2)))
      (else
        (`self.DropItem`)))))

(fn `StoreInOven`
  (params (Hit :type "HitResult Structure"))
  (bind _objectheld (`self.ObjectHeld`))
  (bind _asbp_oven (cast `/Game/Blueprints/BP_Oven` (`.HitActor` (`GameplayStatics.BreakHitResult` Hit))))
  (if (`KismetSystemLibrary.IsValid` _objectheld)
    (if (not (`KismetSystemLibrary.IsValid` (`/Game/Blueprints/BP_Oven.CurrentObject` _asbp_oven)))
      (set `/Game/Blueprints/BP_Oven.CurrentObject` _objectheld _asbp_oven)
      (for _array_element (`self.K2_GetComponentsByClass` _objectheld "/Script/Engine.StaticMeshComponent")
        (bind _asstatic_mesh_component (cast `StaticMeshComponent` _array_element))
        (`PrimitiveComponent.SetSimulatePhysics` _asstatic_mesh_component false)
        (`self.SetActorEnableCollision` _objectheld false))
      (set `self.ObjectHeld` null)
      (else
        (`self.DropItem`)))))

(fn `Tooltips`
  (bind (_locationx _locationy) (`self.GetMousePosition`))
  (bind _tooltip (`self.Tooltip`))
  (bind (_hitresult _didhit) (`self.RayTraceFromMouse` _))
  (if (and _didhit (not (`self.IsStunned`)))
    (bind (_bblockinghit _binitialoverlap _time _distance _location _impactpoint _normal _impactnormal _physmat _hitactor) (`GameplayStatics.BreakHitResult` _hitresult))
    (if (`self.ActorHasTag` _hitactor "Item")
      (bind _asbp_item_base (cast `/Game/Blueprints/Items/BP_ItemBase` _hitactor))
      (bind _amount (`/Game/Blueprints/Items/BP_ItemBase.Amount` _asbp_item_base))
      (if (!= _amount 0)
        (`Widget.SetVisibility` _tooltip "Visible")
        (set `TextBlock.Text` (`KismetTextLibrary.Conv_StringToText` (`KismetStringLibrary.Concat_StrStr` (`KismetStringLibrary.Conv_IntToString` _amount) " " (`/Game/Blueprints/Items/BP_ItemBase.AmountUnit` _asbp_item_base))) (`/Game/Widgets/BP_AmountTooltip.Amount` _tooltip))
        (set `TextBlock.Text` (`KismetTextLibrary.Conv_StringToText` (`/Game/Blueprints/Items/BP_ItemBase.Name` _asbp_item_base)) (`/Game/Widgets/BP_AmountTooltip.Name` _tooltip))
        (`UserWidget.SetPositionInViewport` _tooltip (`KismetMathLibrary.MakeVector2D` _locationx _locationy) true)
        (else
          (`Widget.SetVisibility` _tooltip "Hidden" :!label _label)))
      (else
        (goto _label)))
    (else
      (goto _label))))

(fn `UserConstructionScript`)