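; BP_Bowl is a mixing bowl that tracks ingredient amounts and turns them into dough.
; Each Tick scans the Amounts map and, when none is zero, moves the camera controller's tutorial from "Put Stuff in Bowl" to MixIt with a French right-click-to-mix prompt.
; CreateDough hides the honey, salt, water, yeast and flour components, shows StuffInBowl, copies Amounts to DoughAmounts and sets HasDough.
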(event `self.ReceiveTick`
  (params (DeltaSeconds :type "Float (single-precision)"))
  (set `self.TutorialWasValid` true)
  (bind _values (`BlueprintMapLibrary.Map_Values` (`self.Amounts`)))
  (for _array_element _values
    (if (== _array_element 0)
      (set `self.TutorialWasValid` false)
      (break)))
  (if (`self.TutorialWasValid`)
    (bind _asbp_camera_controller (cast `/Game/Blueprints/Player/BP_CameraController` (`GameplayStatics.GetPlayerController` 0)))
    (switch `/Game/Blueprints/Player/TutorialEnum` (`/Game/Blueprints/Player/BP_CameraController.TutorialState` _asbp_camera_controller)
      (:`NewEnumerator7`
        (`/Game/Blueprints/Player/BP_CameraController.InitiateDialogue` _asbp_camera_controller (`|MakeArray` "Maintenant, faites un clic droit sur le bol pour mélanger les ingrédients.") false 0 0.0)
        (set `/Game/Blueprints/Player/BP_CameraController.TutorialState` "NewEnumerator13" _asbp_camera_controller)))))

(fn `CreateDough`
  (`SceneComponent.SetVisibility` (`self.Honey`) false false)
  (`SceneComponent.SetVisibility` (`self.Salt`) false false)
  (`SceneComponent.SetVisibility` (`self.Water`) false false)
  (`SceneComponent.SetVisibility` (`self.Yeast`) false false)
  (`SceneComponent.SetVisibility` (`self.Flour`) false false)
  (`SceneComponent.SetVisibility` (`self.stuff_in_bowl`) true false)
  (set `self.DoughAmounts` (`self.Amounts`))
  (set `self.HasDough` true))

(fn `UserConstructionScript`)