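; BP_Fridge is a fridge Blueprint that draws a referenced object, CurrentObject, toward a spot offset from itself.
; Each Tick, while that object is valid, TInterpTo eases its transform toward the fridge's rotation and a point forward on world X and below the fridge, keeping its scale.
; The offset ignores the fridge's rotation, and nothing in this file assigns CurrentObject.
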(event `self.ReceiveTick`
  (params (DeltaSeconds :type "Float (single-precision)"))
  (bind _returnvalue (`self.GetTransform`))
  (bind _currentobject (`self.CurrentObject`))
  (if (`KismetSystemLibrary.IsValid` _currentobject)
    (`self.K2_SetActorTransform` _currentobject (`KismetMathLibrary.TInterpTo` (`self.GetTransform` _currentobject) (`KismetMathLibrary.MakeTransform` (`KismetMathLibrary.MakeVector` (+ (.x (.location _returnvalue)) 100.0) (.y (.location _returnvalue)) (+ (.z (.location _returnvalue)) -200.0)) (.rotation _returnvalue) (.scale (`self.GetTransform` _currentobject))) DeltaSeconds 5.0) false false)))

(fn `UserConstructionScript`)