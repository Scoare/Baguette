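; BP_Chef is a chef shown on a Plane component whose look reflects the player's hunger.
; Each tick it oscillates the plane's Y scale with a sine of the frame count, so the animation speed depends on frame rate.
; It also reads Hunger from the player's BP_CameraController and switches between three standing materials at one-third and two-thirds thresholds.
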(event `self.ReceiveTick`
  (params (DeltaSeconds :type "Float (single-precision)"))
  (bind _plane (`self.Plane`))
  (bind _plane_2 (`self.Plane`))
  (bind (_returnvalue_x _returnvalue_y _returnvalue_z) (`KismetMathLibrary.BreakVector` (`SceneComponent.K2_GetComponentScale` _plane_2)))
  (`SceneComponent.SetWorldScale3D` _plane_2 (`KismetMathLibrary.MakeVector` _returnvalue_x (+ (`KismetMathLibrary.DegSin` (* (`KismetMathLibrary.Conv_Int64ToDouble` (`KismetSystemLibrary.GetFrameCount`)) 1.75)) 10.0) _returnvalue_z))
  (bind _asbp_camera_controller (cast `/Game/Blueprints/Player/BP_CameraController` (`GameplayStatics.GetPlayerController` 0)))
  (bind _hunger (`/Game/Blueprints/Player/BP_CameraController.Hunger` _asbp_camera_controller))
  (if (> _hunger 0.66)
    (`PrimitiveComponent.SetMaterial` _plane 0 "/Game/Images/chef/standing_Mat.standing_Mat")
    (elif (> _hunger 0.33)
      (`PrimitiveComponent.SetMaterial` _plane 0 "/Game/Images/chef/standing1_Mat.standing1_Mat")
      (else
        (`PrimitiveComponent.SetMaterial` _plane 0 "/Game/Images/chef/standing2_Mat.standing2_Mat")))))

(fn `UserConstructionScript`)