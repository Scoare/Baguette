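; Base item actor that deposits itself into a bowl when it overlaps a BP_Bowl.
; If the bowl's Amounts map already has a key matching ItemType, it adds its Amount to that entry and destroys itself.
; It then reveals the child component of the bowl's StaticMesh whose object name matches ItemType, so item types and component names are linked by name.
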(event `self.ReceiveActorBeginOverlap`
  (params (OtherActor :type "Actor Object Reference"))
  (bind _itemtype (`self.ItemType`))
  (if (== (`GameplayStatics.GetObjectClass` OtherActor) "/Game/Blueprints/BP_Bowl.BP_Bowl_C")
    (bind _asbp_bowl (cast `/Game/Blueprints/BP_Bowl` OtherActor))
    (bind _amounts (`/Game/Blueprints/BP_Bowl.Amounts` _asbp_bowl))
    (bind _keys (`BlueprintMapLibrary.Map_Keys` _amounts))
    (bind _values (`BlueprintMapLibrary.Map_Values` _amounts))
    (for (_array_element _array_index) _keys
      (if (`KismetStringLibrary.EqualEqual_StrStr` _array_element _itemtype)
        (`BlueprintMapLibrary.Map_Remove` _amounts _array_element)
        (`BlueprintMapLibrary.Map_Add` _amounts _array_element (+ (`|GetArrayItem` _values _array_index) (`self.Amount`)))
        (`self.K2_DestroyActor`)
        (for _array_element_2 (`SceneComponent.GetChildrenComponents` (`/Game/Blueprints/BP_Bowl.StaticMesh` _asbp_bowl) false)
          (if (`KismetStringLibrary.EqualEqual_StrStr` (`KismetSystemLibrary.GetObjectName` _array_element_2) _itemtype)
            (`SceneComponent.SetVisibility` _array_element_2 true false)
            (break)))
        (break)))))

(fn `UserConstructionScript`)