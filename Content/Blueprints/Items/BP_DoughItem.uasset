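; BP_DoughItem is a dough item whose baguette appearance changes with how long it has been in the oven.
; Each Tick compares TimeInOven against two thresholds, swapping the mesh material to cooked at the lower one and to fried at the higher one.
; The file only reads TimeInOven, and BeginPlay and the construction script add no logic of their own.
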(event `self.ReceiveTick`
  (params (DeltaSeconds :type "Float (single-precision)"))
  (bind _mesh (`self.Mesh`))
  (bind _timeinoven (`self.TimeInOven`))
  (`parent.ReceiveTick` DeltaSeconds)
  (if (>= _timeinoven 1.0)
    (`PrimitiveComponent.SetMaterial` _mesh 0 "/Game/Models/Baguette/M_BaguetteFried.M_BaguetteFried")
    (elif (>= _timeinoven 0.5)
      (`PrimitiveComponent.SetMaterial` _mesh 0 "/Game/Models/Baguette/M_BaguetteCooked.M_BaguetteCooked"))))

(fn `UserConstructionScript`
  (`parent.UserConstructionScript`))